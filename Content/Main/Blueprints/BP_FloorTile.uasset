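; BP_FloorTile is a floor segment that keeps a track extending as the main character moves along it.
; On construction it randomly spawns either an obstacle at the middle, left or right spawn point, or a batch of coins scattered within CoinArea, as child actors.
; When the character overlaps EndTrigger, it asks BP_MainGameMode to add a tile, then destroys itself after a short delay.
; GetAttachTransform exposes the AttachPoint world transform.
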(event `self.EndTrigger.OnComponentBeginOverlap`
  (params (OverlappedComponent :type "PrimitiveComponent Object Reference") (OtherActor :type "Actor Object Reference") (OtherComp :type "PrimitiveComponent Object Reference") (OtherBodyIndex :type Integer) (bFromSweep :type Boolean) (SweepResult :type "HitResult Structure (by ref)"))
  ; Add & Destroy Floor Tiles
  (cast `/Game/Main/Blueprints/BP_MainCharacter` OtherActor)
  (bind _asbp_main_game_mode (cast `/Game/Main/Blueprints/BP_MainGameMode` (`GameplayStatics.GetGameMode`)))
  (`/Game/Main/Blueprints/BP_MainGameMode.AddFloorTile` _asbp_main_game_mode)
  (`KismetSystemLibrary.Delay` 2.0)
  (`self.K2_DestroyActor`))

(fn `GetAttachTransform`
  (returns (AttachTransform :type "Transform Structure"))
  (return (`SceneComponent.K2_GetComponentToWorld` (`self.AttachPoint`))))

(fn `SetSpawnPoints`
  (set `self.SpawnPoints` (`|MakeArray` (`SceneComponent.GetRelativeTransform` (`self.SpawnPointM`)) (`SceneComponent.GetRelativeTransform` (`self.SpawnPointL`)) (`SceneComponent.GetRelativeTransform` (`self.SpawnPointR`)))))

(fn `SpawnCoins`
  (bind _coinarea (`self.CoinArea`))
  (for _ (range 5)
    (`AddComponent|NODE_AddChildActorComponent-1` :`RelativeTransform` (`KismetMathLibrary.Conv_VectorToTransform` (`KismetMathLibrary.RandomPointInBoundingBox` (`SceneComponent.RelativeLocation` _coinarea) (`BoxComponent.BoxExtent` _coinarea))))))

(fn `SpawnObstacle`
  (bind _spawnpoints (`self.SpawnPoints`))
  (`AddComponent|NODE_AddChildActorComponent-0` :`RelativeTransform` (`|GetArrayItem` _spawnpoints (`KismetMathLibrary.RandomIntegerInRange` 0 (`KismetArrayLibrary.Array_LastIndex` _spawnpoints)))))

(fn `UserConstructionScript`
  (`self.SetSpawnPoints`)
  (switch `int` (`KismetMathLibrary.RandomIntegerInRange` 0 1)
    (:`Default`
      (`self.SpawnObstacle` :!label _label))
    (:`0`
      (goto _label))
    (:`1`
      (`self.SpawnCoins`))))