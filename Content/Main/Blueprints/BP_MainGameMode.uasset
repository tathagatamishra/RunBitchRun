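; Main game mode for what looks like an endless-runner style game, handling start-up HUD, intro sound and floor generation.
; On BeginPlay it shows WBP_GameHUD and plays a voice cue at the main character's location.
; It then loops AddFloorTile, chaining each BP_FloorTile spawn to the previous tile's attach transform.
; The loop body also sets half-speed time dilation, restored after a one-second Delay.
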(event `self.ReceiveBeginPlay`
  (bind _returnvalue (`|CreateWidget` "/Game/Main/UI/WBP_GameHUD.WBP_GameHUD_C"))
  (`UserWidget.AddToViewport` _returnvalue 0)
  (bind _returnvalue_2 (`GameplayStatics.GetActorOfClass` "/Game/Main/Blueprints/BP_MainCharacter.BP_MainCharacter_C"))
  (`/Engine/EditorBlueprintResources/StandardMacros.IsValid` _returnvalue_2
    (:`Is Valid`
      (`GameplayStatics.PlaySoundAtLocation` "/Game/Sounds/AhShitHereWeGoAgain_audio_Cue.AhShitHereWeGoAgain_audio_Cue" (`self.K2_GetActorLocation` _returnvalue_2) (struct) 0.1 1.0 0.0 null null null null))
    (:`Is Not Valid`
      _))
  (for _ (range (+ (`self.TileGenerateCount`) 1))
    (`self.AddFloorTile`)
    (`GameplayStatics.SetGlobalTimeDilation` 0.5)
    (`KismetSystemLibrary.Delay` 1.0)
    (`GameplayStatics.SetGlobalTimeDilation` 1.0)))

(fn `AddFloorTile`
  (bind _returnvalue (`|SpawnActorFromClass` "/Game/Main/Blueprints/BP_FloorTile.BP_FloorTile_C" (`self.NextSpawnPoint`) "Undefined" "MultiplyWithRoot" null null))
  (bind _asbp_floor_tile (cast `/Game/Main/Blueprints/BP_FloorTile` _returnvalue))
  (bind _attachtransform (`/Game/Main/Blueprints/BP_FloorTile.GetAttachTransform` _asbp_floor_tile))
  (set `self.NextSpawnPoint` _attachtransform))

(fn `UserConstructionScript`)